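; BP_SpawnManager is a spawner that places BP_Clown or BP_PNJ actors in the game.
; BeginPlay caches the player and starts two looping timers, one at the spawn interval and one at the level interval.
; PNJOrClown rolls a random number against LuckClown, picks a random target location, and spawns only outside a minimum player distance.
; AugmentLevel conditionally raises clown odds and resets a very low spawn interval.
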(event Custom|Spawn
  (params (Spawn%20Transform%20Location :type Vector))
  (Game|SpawnActorfromClass (select (<= (Variables|Default|GetRandomClown) (Variables|Default|GetLuckClown)) "/Game/BP_Clown.BP_Clown_C" "/Game/BP_PNJ.BP_PNJ_C") (Math|Transform|MakeTransform Spawn%20Transform%20Location "0, 0, 0" "1.000000,1.000000,1.000000") "Undefined" "MultiplyWithRoot" 0 0))

(event Custom|PNJOrClown
  (Variables|Default|SetRandomClown (Math|Random|RandomIntegerinRange 0 100))
  (CallFunction|LocationCalcul))

(event Custom|LocationCalcul
  (bind _output_get (Variables|Default|SetSpawnLocation (.OutItem (Utilities|Array|Random (Variables|Default|GetTargetSpawn)))))
  (if (not (< (Math|Vector|Distance(Vector) (Transformation|GetActorLocation (Variables|Default|GetPlayerRef)) _output_get) (Variables|Default|GetDistanceMin)))
    (CallFunction|Spawn _output_get)))

(event Custom|AugmentLevel
  (Development|PrintString "Hello")
  (Utilities|FlowControl|Sequence
    (:then_0
      (if (< (Variables|Default|GetRandomClown) 60)
        (Variables|Default|SetLuckClown (+ (Variables|Default|GetLuckClown) 3))))
    (:then_1
      (if (< (Variables|Default|GetNewSpawn) 0.1)
        (Variables|Default|SetNewSpawn (* (Variables|Default|GetMaxNewSpawn) 0.95))))))

(event Custom|SetVar
  (Variables|Default|SetNewSpawn (Variables|Default|GetMaxNewSpawn)))

(event EventBeginPlay
  (bind _asbp_chara_player (Utilities|Casting|CastToBP_CharaPlayer (Game|Player|GetPlayerPawn 0)))
  (Variables|Default|SetPlayerRef _asbp_chara_player)
  (Utilities|Time|SetTimerbyEvent (EventDispatchers|CreateEvent :!event Custom|PNJOrClown) (Variables|Default|GetNewSpawn) true)
  (Utilities|Time|SetTimerbyEvent (EventDispatchers|CreateEvent :!event Custom|AugmentLevel) (Variables|Default|GetTimelevel) true))

(fn ConstructionScript)