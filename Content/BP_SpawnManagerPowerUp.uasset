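; Spawn manager that places random power-ups (range, attack speed or projectile speed) in the level.
; BeginPlay caches the player character and starts a looping timer on the NewSpawn interval.
; LocationCalcul picks a random TargetSpawn location and skips it, without retrying, if the player is closer than DistanceMin.
; Otherwise, Spawn creates one of the three power-up classes slightly above that location.
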(event Custom|Spawn
  (params (Spawn%20Transform%20Location :type Vector))
  (Game|SpawnActorfromClass (Utilities|Select :Index (Math|Random|RandomIntegerinRange 0 2) :Option%200 "/Game/BP_Range.BP_Range_C" :Option%201 "/Game/BP_AttackSpeed.BP_AttackSpeed_C" :Option%202 "/Game/BP_SpeedProjectile.BP_SpeedProjectile_C") (Math|Transform|MakeTransform (+ Spawn%20Transform%20Location "0.000000,0.000000,100.000000") "0, 0, 0" "1.000000,1.000000,1.000000") "Undefined" "MultiplyWithRoot" 0))

(event Custom|LocationCalcul
  (bind _output_get (Variables|Default|SetSpawnLocation (.OutItem (Utilities|Array|Random (Variables|Default|GetTargetSpawn)))))
  (if (not (< (Math|Vector|Distance(Vector) (Transformation|GetActorLocation (Variables|Default|GetPlayerRef)) _output_get) (Variables|Default|GetDistanceMin)))
    (CallFunction|Spawn _output_get)))

(event EventBeginPlay
  (bind _asbp_chara_player (Utilities|Casting|CastToBP_CharaPlayer (Game|Player|GetPlayerPawn 0)))
  (Variables|Default|SetPlayerRef _asbp_chara_player)
  (Utilities|Time|SetTimerbyEvent (EventDispatchers|CreateEvent :!event Custom|LocationCalcul) (Variables|Default|GetNewSpawn) true))

(fn ConstructionScript)