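; BP_Clown is an actor, likely an enemy, that gains PV over time and can drop an item when destroyed.
; A looping timer started on BeginPlay increments PV by one at each interval.
; On destruction, if the Characte reference is valid, a weighted coin flip decides whether to spawn either BP_SpeedProjectile or BP_AttackSpeed, picked at random, at the clown's transform.
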(event Custom|Augment
  (Math|Integer|IncrementInt (Variables|Default|GetPV)))

(event EventBeginPlay
  (Utilities|Time|SetTimerbyEvent (delegate Custom|Augment) (Variables|Default|GetTime) true))

(event EventDestroyed
  (Utilities|IsValid (Variables|Default|GetCharacte)
    (:Is%20Valid
      (if (Math|Random|RandomBoolwithWeight 0.5)
        (Game|SpawnActorfromClass (Utilities|Select :Index (Math|Random|RandomIntegerinRange 0 1) :Option%200 "/Game/BP_SpeedProjectile.BP_SpeedProjectile_C" :Option%201 "/Game/BP_AttackSpeed.BP_AttackSpeed_C") (Transformation|GetActorTransform) "Undefined" "MultiplyWithRoot" 0 0)))))

(fn ConstructionScript)